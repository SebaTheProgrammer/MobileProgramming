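; BP_HealthPickup is a one-time health pickup that adds AddHP to the HP of a BP_ThirdPersonCharacter on contact.
; A Box overlap event casts the overlapping actor, raises its HP directly with no clamp in this graph, and sets a HasPickedUp flag against repeat triggers.
; It then hides its components, plays a 2D battery pickup sound and destroys itself.
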(event OnComponentBeginOverlap(Box)
  (params (OverlappedComponent :type Primitive%20Component%20Object%20Reference) (OtherActor :type Actor%20Object%20Reference) (OtherComp :type Primitive%20Component%20Object%20Reference) (OtherBodyIndex :type Integer) (bFromSweep :type Boolean) (SweepResult :type Hit%20Result%20Structure%20%28by%20ref%29))
  (if (not (Variables|Default|GethasPickedUp))
    (bind _asbp_third_person_character (Utilities|Casting|CastToBP_ThirdPersonCharacter OtherActor))
    (Variables|/Game/ThirdPerson/Blueprints/BP_ThirdPersonCharacter.BP_ThirdPersonCharacter_C|SetHP _asbp_third_person_character (+ (Variables|/Game/ThirdPerson/Blueprints/BP_ThirdPersonCharacter.BP_ThirdPersonCharacter_C|GetHP _asbp_third_person_character) (Variables|Default|GetaddHP)))
    (Variables|Default|SethasPickedUp true)
    (Rendering|SetVisibility (Variables|Default|GetDefaultSceneRoot) false true)
    (Audio|PlaySound2D "/Game/STW/Audio/Effects/BatteryPickup.BatteryPickup" 1.0 1.0 0.0 0 0)
    (Actor|DestroyActor)))

(fn ConstructionScript)