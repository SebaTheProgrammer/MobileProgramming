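; Sound handler Blueprint that plays random background songs throughout a level.
; After a startup delay on BeginPlay, PlaySong plays a random track from the BgSongs array as 2D sound at BgVolume.
; It then waits a random time between configurable min and max delays and calls itself again, looping indefinitely without checking whether the previous song has finished.
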(event Custom|PlaySong
  (Audio|PlaySound2D (.OutItem (Utilities|Array|Random (Variables|Default|GetbgSongs))) (Variables|Default|GetbgVolume) 1.0 0.0 0 0)
  (Utilities|FlowControl|Delay (Math|Random|RandomFloatinRange (Variables|Default|GetminDelayNextSong) (Variables|Default|GetmaxDelayNextSong)))
  (CallFunction|PlaySong))

(event EventBeginPlay
  (Utilities|FlowControl|Delay 2e+01)
  (CallFunction|PlaySong))

(fn ConstructionScript)