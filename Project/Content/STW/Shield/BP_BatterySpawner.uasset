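; BP_BatterySpawner repeatedly spawns P_Battery actors at random navigable points around itself.
; After a startup delay, CalculateSpawnPoint waits a random interval, spawns a battery, then calls itself again indefinitely.
; A zero-delay retry loop rejects random points inside a central exclusion box sized by MinSpawnRadius, but the spawn draws a fresh random point instead of reusing the tested one.
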(event Custom|CalculateSpawnPoint
  (bind _minspawnradius (Variables|Default|GetminSpawnRadius))
  (bind _defaultsceneroot (Variables|Default|GetDefaultSceneRoot))
  (bind _spawnradius (Variables|Default|GetspawnRadius))
  (bind _returnvalue (Transformation|GetWorldLocation _defaultsceneroot))
  (bind _randomlocation (AI|Navigation|GetRandomReachablePointinRadius _returnvalue _spawnradius 0 0))
  (Utilities|FlowControl|Delay (Math|Random|RandomFloatinRange (Variables|Default|GetMINTimeBetweenSpawn) (Variables|Default|GetMAXTimeBetweenSpawn)))
  (Utilities|FlowControl|Delay 0.0 :!label _label)
  (if (Math|Geometry|IsPointinBox _randomlocation (Transformation|GetWorldLocation (Variables|Default|GetDefaultSceneRoot)) (Math|Vector|MakeVector _minspawnradius _minspawnradius _minspawnradius))
    (goto _label)
    (else
      (Game|SpawnActorfromClass "/Game/STW/Shield/P_Battery.P_Battery_C" (Math|Transform|MakeTransform _randomlocation "0, 0, 0" "1.000000,1.000000,1.000000") "AlwaysSpawn" "MultiplyWithRoot" 0 0)
      (CallFunction|CalculateSpawnPoint))))

(event EventBeginPlay
  (Utilities|FlowControl|Delay 1e+01)
  (CallFunction|CalculateSpawnPoint))

(fn ConstructionScript)