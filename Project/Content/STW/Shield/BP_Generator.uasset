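; Shield generator actor that turns batteries from BP_ThirdPersonCharacter into a P_Shield and also spawns ammo crates.
; CanSpawnShield spawns the shield or tops up its HP, capped at 100, then deducts batteries; Tick clears IsOn when HP runs out.
; A box overlap toggles the PRESSE prompt and activation permission while the shield is off.
; A recursive delayed event relocates one BP_Ammo crate among five random points.
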(event OnComponentBeginOverlap(Box)
  (params (OverlappedComponent :type Primitive%20Component%20Object%20Reference) (OtherActor :type Actor%20Object%20Reference) (OtherComp :type Primitive%20Component%20Object%20Reference) (OtherBodyIndex :type Integer) (bFromSweep :type Boolean) (SweepResult :type Hit%20Result%20Structure%20%28by%20ref%29))
  ;[1 1 1] Show 'Press E'
  (Utilities|Casting|CastToBP_ThirdPersonCharacter OtherActor)
  (if (not (Variables|Default|GetisOn))
    (Variables|Default|SetcanActivateShield true)
    (Rendering|SetVisibility (Variables|Default|GetPRESS%20E) true false)))

(event OnComponentEndOverlap(Box)
  (params (OverlappedComponent :type Primitive%20Component%20Object%20Reference) (OtherActor :type Actor%20Object%20Reference) (OtherComp :type Primitive%20Component%20Object%20Reference) (OtherBodyIndex :type Integer))
  ;[1 1 1] Show 'Press E'
  (Utilities|Casting|CastToBP_ThirdPersonCharacter OtherActor)
  (if (not (Variables|Default|GetisOn))
    (Variables|Default|SetcanActivateShield false)
    (Rendering|SetVisibility (Variables|Default|GetPRESS%20E) false false)))

(event Custom|CanSpawnShield
  (params (#Batteries :type Integer))
  (bind _canactivateshield (Variables|Default|GetcanActivateShield))
  (bind __onebat (Variables|Default|Get%25OneBat))
  (bind _returnvalue (* #Batteries __onebat))
  ;[1 1 1] SpawnAndUpdate
  (if (> #Batteries 0)
    (if (Variables|Default|GetisOn)
      (if _canactivateshield
        (CallFunction|AddSHield #Batteries (stale _returnvalue_2))
        (CallFunction|SubstractBatteries))
      (elif _canactivateshield
        (Variables|Default|SethpShield (Math|Conversions|ToFloat(Integer) _returnvalue))
        (if (<= _returnvalue 100)
          _
          (else
            (Variables|Default|SethpShield 1e+02)))
        (bind _returnvalue_2 (Game|SpawnActorfromClass "/Game/STW/Shield/Blue/P_Shield.P_Shield_C" (Math|Transform|MakeTransform (.location (Transformation|GetWorldTransform (Variables|Default|GetDefaultSceneRoot))) "0, 0, 0" "1.000000,1.000000,1.000000") "AlwaysSpawn" "MultiplyWithRoot" 0 (Variables|Default|GethpShield) 0))
        (CallFunction|SubstractBatteries)
        (Variables|Default|SetisOn true)))))

(event Custom|AddShield
  (params (#Batteries :type Integer) (Target :type P%20Shield%20Object%20Reference))
  ;[0.2327 0.4667 1] ShieldLogic
  (if (<= (+ (* #Batteries (Variables|Default|Get%25OneBat)) (Variables|/Game/STW/Shield/Blue/P_Shield.P_Shield_C|GetHP Target)) 1e+02)
    (Variables|/Game/STW/Shield/Blue/P_Shield.P_Shield_C|SetHP Target (Math|Conversions|ToFloat(Integer) (Math|Float|Truncate (+ (* #Batteries (Variables|Default|Get%25OneBat)) (Variables|/Game/STW/Shield/Blue/P_Shield.P_Shield_C|GetHP Target)))))
    (Variables|Default|SethpShield 0.0)
    (else
      (bind _output_get (Variables|Default|SethpShield 1e+02))
      (Variables|/Game/STW/Shield/Blue/P_Shield.P_Shield_C|SetHP Target _output_get))))

(event Custom|SubstractBatteries
  ;[0.2327 0.4667 1] ShieldLogic
  (bind _asbp_third_person_character (Utilities|Casting|CastToBP_ThirdPersonCharacter (Game|GetPlayerCharacter 0)))
  (if (>= (- (Variables|/Game/ThirdPerson/Blueprints/BP_ThirdPersonCharacter.BP_ThirdPersonCharacter_C|Get#batteries _asbp_third_person_character) (/ (Variables|Default|GethpShield) (Variables|Default|Get%25OneBat))) 0.0)
    (Variables|/Game/ThirdPerson/Blueprints/BP_ThirdPersonCharacter.BP_ThirdPersonCharacter_C|Set#batteries _asbp_third_person_character (Math|Float|Truncate (- (Variables|/Game/ThirdPerson/Blueprints/BP_ThirdPersonCharacter.BP_ThirdPersonCharacter_C|Get#batteries _asbp_third_person_character) (/ (Variables|Default|GethpShield) (Variables|Default|Get%25OneBat)))))
    (else
      (Variables|/Game/ThirdPerson/Blueprints/BP_ThirdPersonCharacter.BP_ThirdPersonCharacter_C|Set#batteries _asbp_third_person_character 0))))

(event Custom|SpawnAmmoCrates
  (if (Variables|Default|GethasAmmoCrates)
    _
    (else
      (bind _returnvalue (Game|SpawnActorfromClass "/Game/STW/Player/BP_Ammo.BP_Ammo_C" (Math|Transform|MakeTransform (Transformation|GetWorldLocation (.OutItem (Utilities|Array|Random (Utilities|Array|MakeArray (Variables|Default|GetSpawnPointsAmmoCrate) (Variables|Default|GetSpawnPointsAmmoCrate1) (Variables|Default|GetSpawnPointsAmmoCrate2) (Variables|Default|GetSpawnPointsAmmoCrate3) (Variables|Default|GetSpawnPointsAmmoCrate4))))) "0, 0, 0" "1.000000,1.000000,1.000000") "AlwaysSpawn" "MultiplyWithRoot" 0 0))
      (Variables|Default|SethasAmmoCrates true)))
  (Utilities|FlowControl|Delay (Variables|Default|GetwaitTimeAmmoCrates))
  (Variables|Default|SethasAmmoCrates false)
  (Utilities|IsValid _returnvalue
    (:Is%20Valid
      (Actor|DestroyActor _returnvalue))
    (:Is%20Not%20Valid
      _))
  (CallFunction|SpawnAmmoCrates))

(event EventTick
  (params (DeltaSeconds :type Float%20%28single-precision%29))
  ;[1 1 1] SpawnAndUpdate
  (if (Variables|Default|GetisOn)
    (if (<= (Variables|/Game/STW/Shield/Blue/P_Shield.P_Shield_C|GetHP (stale Custom|CanSpawnShield _returnvalue_2)) 0.0)
      (Variables|Default|SetisOn false))))

(event EventBeginPlay
  ;[1 1 1] SpawnAndUpdate
  (Rendering|SetVisibility (Variables|Default|GetPRESS%20E) false false)
  (CallFunction|SpawnAmmoCrates))

(fn ConstructionScript)