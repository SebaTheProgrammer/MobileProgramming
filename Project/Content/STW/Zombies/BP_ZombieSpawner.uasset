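; Zombie spawner that continuously adds wandering AI zombies at random reachable navmesh points around a spot ahead of or behind the player.
; A self-calling delayed loop starts after BeginPlay, with a FlipFlop alternating sides.
; NextWave switches to randomized wave timing and re-triggers the loop, while StopWave restores the peace interval.
; Once CanSpawnBiggys is called, a one-in-five roll adds an extra spawn, alternating big and normal zombies.
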(event Custom|CalculateSpawnPoint
  ;[1 1 1] Main
  (if (Variables|Default|GetHigherDensity)
    (Utilities|FlowControl|Delay (Math|Random|RandomFloatinRange (Variables|Default|GetMINTimeBetweenSpawn) (Variables|Default|GetMAXTimeBetweenSpawn)))
    (else
      (Utilities|FlowControl|Delay (Variables|Default|GetpeaceSpawnTime))))
  (Utilities|FlowControl|FlipFlop
    (:A
      (CallFunction|Spawn -1.0))
    (:B
      (CallFunction|Spawn 1.0)))
  (if (Variables|Default|GetcanSpawnBig)
    (CallFunction|CalculateSpawnPoint)
    (if (== 0 (Math|Random|RandomInteger 5))
      (Utilities|FlowControl|FlipFlop
        (:A
          (CallFunction|SpawnBig 1.0))
        (:B
          (CallFunction|Spawn -1.0))))
    (else
      (CallFunction|CalculateSpawnPoint))))

(event Custom|NextWave
  (Variables|Default|SetHigherDensity true)
  (CallFunction|CalculateSpawnPoint))

(event Custom|StopWave
  (Variables|Default|SetHigherDensity false))

(event Custom|Spawn
  (params (forwardVector* :type Float%20%28double-precision%29))
  ;[1 1 1] Normals
  (bind _randomlocation (CallFunction|CalculatePoint forwardVector*))
  (AI|SpawnAIFromClass "/Game/STW/Zombies/BP_Zombie.BP_Zombie_C" "/Game/STW/Zombies/Behaviour/BT_Wander.BT_Wander" _randomlocation "0, 0, 0" false 0))

(event Custom|CanSpawnBiggys
  (Variables|Default|SetcanSpawnBig true))

(event Custom|SpawnBig
  (params (ForwardVectorMultiplier :type Float%20%28double-precision%29))
  ;[1 1 1] Big
  (bind _randomlocation (CallFunction|CalculatePoint ForwardVectorMultiplier))
  (AI|SpawnAIFromClass "/Game/STW/Zombies/BP_BigZombies.BP_BigZombies_C" "/Game/STW/Zombies/Behaviour/BT_Wander.BT_Wander" _randomlocation "0, 0, 0" false 0))

(event EventBeginPlay
  (Utilities|FlowControl|Delay 1e+01)
  (CallFunction|CalculateSpawnPoint)
  (Variables|Default|SetcanSpawnBig false))

(fn ConstructionScript)

(fn CalculatePoint
  (params (ForwardVectorMultiplier :type Float%20%28double-precision%29))
  (bind _returnvalue (Game|Player|GetPlayerPawn 0))
  (return (.RandomLocation (AI|Navigation|GetRandomReachablePointinRadius (+ (* (Transformation|GetActorForwardVector _returnvalue) (* (Variables|Default|GetspawnDistance) ForwardVectorMultiplier)) (Transformation|GetActorLocation _returnvalue)) (Math|Random|RandomFloatinRange (Variables|Default|GetminSpawnRadius) (Variables|Default|GetmaxSpawnRadius)) 0 0))))